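; Player controller for a furniture placement game that creates the HUD, spawns the selected furniture at a given location, and toggles UI visibility.
; Saving appends each Furniture actor's class, transform and first material vector parameter as color to a BP_FurnitureSave object, then writes it to a slot.
; Loading destroys all existing furniture, then respawns the saved pieces and reapplies their "Color" parameter.
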(event `self.ReceiveBeginPlay`
  (bind _returnvalue (`|CreateWidget` "/Game/UI/UI_HUD.UI_HUD_C" self))
  (bind _output_get (set `self.HUD` _returnvalue))
  (`UserWidget.AddToViewport` _output_get 0)
  (bind _returnvalue_2 (`GameplayStatics.CreateSaveGameObject` "/Game/Blueprints/BP_FurnitureSave.BP_FurnitureSave_C"))
  (set `self.FurnitureSave` _returnvalue_2))

(event `self.PlaceFurnitureAtClickLocation`
  (params (Location :type "Vector Structure (by ref)"))
  (bind _hud (`self.HUD`))
  (bind (_output_name _output_furniture) (break `/Game/DataSets/STR_Spawnable` (`|GetArrayItem` (`/Game/UI/UI_HUD.SpawnableList` _hud) (`/Game/UI/UI_HUD.SpawnableIndex` _hud))))
  (`|SpawnActorFromClass` _output_furniture (`KismetMathLibrary.MakeTransform` Location) "Undefined" "OverrideRootScale" null null))

(event `self.CloseColorWheel`
  (`/Game/UI/UI_HUD.SetModeToSelecting` (`self.HUD`)))

(event `BeginSave`
  (bind _furnituresave (`self.FurnitureSave`))
  (bind _outactors (`GameplayStatics.GetAllActorsOfClass` "/Script/Sneakybox_Interior.Furniture"))
  (for _array_element _outactors
    (`self.AddFurnitureInfoToArray` _array_element))
  (`GameplayStatics.SaveGameToSlot` _furnituresave (`/Game/Blueprints/BP_FurnitureSave.SaveSlotName` _furnituresave) (`/Game/Blueprints/BP_FurnitureSave.UserIndex` _furnituresave)))

(event `BeginLoad`
  (bind _furnituresave (`self.FurnitureSave`))
  (bind _returnvalue (`GameplayStatics.LoadGameFromSlot` (`/Game/Blueprints/BP_FurnitureSave.SaveSlotName` _furnituresave) (`/Game/Blueprints/BP_FurnitureSave.UserIndex` _furnituresave)))
  (bind _asbp_furniture_save (cast `/Game/Blueprints/BP_FurnitureSave` _returnvalue))
  (set `self.FurnitureSave` _asbp_furniture_save)
  (bind _outactors (`GameplayStatics.GetAllActorsOfClass` "/Script/Sneakybox_Interior.Furniture"))
  (for _array_element _outactors
    (`self.K2_DestroyActor` _array_element))
  (`self.PlaceLoadedFurniture`))

(event `InputAction|ToggleUI`
  (params (Key :type "Key Structure"))
  (bind _hud (`self.HUD`))
  (:`Pressed`
    (`/Engine/EditorBlueprintResources/StandardMacros.FlipFlop`
      (:`A`
        (`Widget.SetVisibility` _hud "Hidden"))
      (:`B`
        (`Widget.SetVisibility` _hud "Visible")))))

(fn `AddFurnitureInfoToArray`
  (params (Furniture :type "Furniture Object Reference"))
  (bind _asmaterial_instance (cast `MaterialInstance` (`PrimitiveComponent.GetMaterial` (`Furniture.Mesh` Furniture) 0)))
  (bind (_output_parameterinfo _output_parametervalue) (break `VectorParameterValue` (`|GetArrayItem` (`MaterialInstance.VectorParameterValues` _asmaterial_instance))))
  (`KismetArrayLibrary.Array_Add` (`/Game/Blueprints/BP_FurnitureSave.FurnitureInfo` (`self.FurnitureSave`)) (make `/Game/DataSets/STR_Loadable` (`GameplayStatics.GetObjectClass` Furniture) (`self.GetTransform` Furniture) _output_parametervalue)))

(fn `PlaceLoadedFurniture`
  (for _array_element (`/Game/Blueprints/BP_FurnitureSave.FurnitureInfo` (`self.FurnitureSave`))
    (bind _returnvalue (`|SpawnActorFromClass` (break `/Game/DataSets/STR_Loadable` _array_element) (`.FurnitureTransform_6_6948CF2449F5F361D3439AABED523501` (break `/Game/DataSets/STR_Loadable` _array_element)) "Undefined" "OverrideRootScale" null null))
    (`MeshComponent.SetVectorParameterValueOnMaterials` (`Furniture.Mesh` _returnvalue) "Color" (`KismetMathLibrary.Conv_LinearColorToVector` (`.FurnitureColor_9_A1994BE446BC686BAA61F087935032F7` (break `/Game/DataSets/STR_Loadable` _array_element))))))

(fn `UserConstructionScript`)